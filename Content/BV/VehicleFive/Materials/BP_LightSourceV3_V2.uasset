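; Light source actor that acts as a stimulus for nearby BP_CarV2_2 cars.
; Every Tick it runs a multi-sphere object trace around itself, with persistent debug drawing, and passes its location to MoveForward on hit cars whose names contain "V2".
; GetThrottleInputs derives left and right throttles from the stored location's distance to world origin, using different falloff ranges, but is not called here.
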(event Custom|ScrubTrace
  ;[1 1 1] Scrub Trace for Car and throttle input
  (bind _output_get (Variables|Default|SetmyLocation (Transformation|GetActorLocation)))
  (bind _outhits (Collision|MultiSphereTraceForObjects _output_get _output_get 3e+03 (Variables|Default|GetObject%20Types) false 0 "Persistent" true "(R=1.000000,G=0.000000,B=0.000000,A=1.000000)" "(R=1.000000,G=0.137221,B=0.081479,A=1.000000)"))
  (for _array_element _outhits
    (if (Utilities|String|Contains (Utilities|GetDisplayName (.HitActor (Collision|BreakHitResult _array_element))) "V2")
      (bind _asbp_car_v2_2 (Utilities|Casting|CastToBP_CarV2_2 (.HitActor (Collision|BreakHitResult _array_element))))
      (Default|MoveForward _asbp_car_v2_2 (Variables|Default|GetmyLocation)))))

(event EventTick
  (params (DeltaSeconds :type Float%20%28single-precision%29))
  (CallFunction|ScrubTrace))

(fn ConstructionScript)

(fn GetThrottleInputs
  (return (- 1.0 (Math|Float|NormalizetoRange (Math|Float|NormalizetoRange (/ (Math|Vector|VectorLength (- "" (Variables|Default|GetmyLocation))) 7.5e+03) 0.0 1.0) 0.0 1.0)) (- 1.0 (Math|Float|NormalizetoRange (Math|Float|NormalizetoRange (/ (Math|Vector|VectorLength (- "" (Variables|Default|GetmyLocation))) 3e+03) 0.0 1.0) 0.0 1.0))))