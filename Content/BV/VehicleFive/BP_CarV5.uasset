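; Self-driving vehicle Blueprint that steers and throttles itself in response to nearby actors with "source" in their display name.
; Each tick a debug-drawn sphere trace finds sources, feeding sensor-to-source distance through a NeuralComponent for throttle.
; Steering scales the world look-at yaw toward the source, without subtracting the car's heading.
; An optional widget shows live values; the ReLU, sigmoid and step helpers are uncalled in these graphs.
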(event Custom|ScrubTrace
  (bind _returnvalue (Transformation|GetActorLocation))
  (bind _outhits (Collision|MultiSphereTraceForObjects _returnvalue _returnvalue 2.8e+03 (Variables|Default|GetObject%20Types) false 0 "ForDuration" true "(R=0.088195,G=1.000000,B=0.100112,A=1.000000)" "(R=0.263167,G=1.000000,B=0.093465,A=1.000000)" 1.0))
  (for _array_element _outhits
    (if (Utilities|String|Contains (Utilities|GetDisplayName (.HitActor (Collision|BreakHitResult _array_element))) "source")
      (Variables|Default|SethitLocation (Transformation|GetActorLocation (.HitActor (Collision|BreakHitResult _array_element))))
      (bind (_throttle _weight) (CallFunction|GetthrottleInputs))
      (bind _steering (CallFunction|GetSteeringAngle))
      (Variables|Default|SetWeight _weight)
      (bind _output_get (Variables|Default|SetAngle _steering))
      (Class|ChaosVehicleMovementComponent|SetSteeringInput (Variables|Default|GetVehicleMovementComponent) _output_get)
      (bind _output_get_2 (Variables|Default|SetThrottle (* _throttle (Variables|Default|GetThrottleSmoother))))
      (Class|ChaosVehicleMovementComponent|SetThrottleInput (Variables|Default|GetVehicleMovementComponent) _output_get_2)
      ;[1 1 1] WidgetUpdate
      (if (Variables|Default|Getinfo?)
        (if (Variables|Default|GetinfoUp)
          _
          (else
            (bind _returnvalue_2 (UserInterface|CreateWidget "/Game/BV/UI/UW_CarInfo.UW_CarInfo_C" (Game|GetPlayerController 0)))
            (bind _output_get_3 (Variables|Default|SetcarinfoWidget _returnvalue_2))
            (UserInterface|Viewport|AddtoViewport _output_get_3 0)
            (Variables|Default|SetinfoUp true)))
        (Variables|/Script/UMG.TextBlock|SetText (Variables|/Game/BV/UI/UW_CarInfo.UW_CarInfo_C|GetThrottle (Variables|Default|GetcarinfoWidget)) (Utilities|Text|ToText(Float) (Variables|Default|GetThrottle) "HalfToEven"))
        (Variables|/Script/UMG.TextBlock|SetText (Variables|/Game/BV/UI/UW_CarInfo.UW_CarInfo_C|GetAngle (Variables|Default|GetcarinfoWidget)) (Utilities|Text|ToText(Float) (Variables|Default|GetAngle) "HalfToEven"))
        (Variables|/Script/UMG.TextBlock|SetText (Variables|/Game/BV/UI/UW_CarInfo.UW_CarInfo_C|GetNMR (Variables|Default|GetcarinfoWidget)) (Utilities|Text|ToText(Integer) (Variables|Default|GetNMR)))
        (Variables|/Script/UMG.TextBlock|SetText (Variables|/Game/BV/UI/UW_CarInfo.UW_CarInfo_C|GetWeight (Variables|Default|GetcarinfoWidget)) (Utilities|Text|ToText(Float) (Variables|Default|GetWeight) "HalfToEven"))
        (Variables|/Script/UMG.TextBlock|SetText (Variables|/Game/BV/UI/UW_CarInfo.UW_CarInfo_C|GetVehicleName (Variables|Default|GetcarinfoWidget)) (Utilities|Text|ToText(Name) (Variables|Default|GetCarname)))
        (else
          (bind _carinfowidget (Variables|Default|GetcarinfoWidget)
            (:then
              (Widget|RemovefromParent _carinfowidget)
              (Variables|Default|SetinfoUp false))
            (:else)))))))

(event EventTick
  (params (DeltaSeconds :type Float%20%28single-precision%29))
  (Variables|Default|Setcar%20location (Transformation|GetActorLocation))
  (CallFunction|ScrubTrace))

(fn ConstructionScript)

(fn GetSensorinput
  (params (Sensor :type Vector))
  (bind _hitlocation (Variables|Default|GethitLocation))
  (bind _returnvalue (- _hitlocation Sensor))
  (bind _returnvalue_2 (Math|Vector|VectorLength _returnvalue))
  ;[1 1 1] Get Sensory input
  (bind (_out _weight) (Default|GetThrottleInput (Variables|Default|GetNeuralComponent) (/ (Math|Float|NormalizetoRange (/ _returnvalue_2 3e+01) 0.0 1.0) 6e+01) _returnvalue_2))
  (return _out _weight))

(fn GetthrottleInputs
  (bind (_sensorout _weight) (CallFunction|GetSensorinput (Transformation|GetWorldLocation (Variables|Default|GetExhiSensor))))
  (return _sensorout _weight))

(fn GetSteeringAngle
  (return (* (Variables|Default|GetSteeringSmoother) (/ (.yaw (Math|Rotator|FindLookatRotation (Variables|Default|Getcar%20location) (Variables|Default|GethitLocation))) 3.6e+02))))

(fn ReluFunction
  (params (input :type Float%20%28double-precision%29) (Threshold :type Float%20%28double-precision%29))
  (if (< input Threshold)
    (return 0.0)
    (else
      (return input))))

(fn SigmoidFunction
  (params (Input :type Float%20%28double-precision%29))
  (bind _returnvalue (* Input -1.0))
  (bind _returnvalue_2 (Class|KismetMathLibrary|Exp _returnvalue))
  (bind _returnvalue_3 (+ 1.0 _returnvalue_2))
  (bind _returnvalue_4 (/ 1.0 _returnvalue_3))
  (Development|PrintText (Utilities|Text|FormatText "Input {in} output {out}" Input _returnvalue_4))
  (return _returnvalue_4))

(fn StepFunction
  (params (Input :type Float%20%28double-precision%29) (ThresholdA :type Float%20%28double-precision%29) (ThresholdB :type Float%20%28double-precision%29))
  (if (<= Input ThresholdA)
    (Development|PrintString (Utilities|String|ToString(Float) ThresholdA))
    (return ThresholdA)
    (elif (>= Input ThresholdB)
      (Development|PrintString (Utilities|String|ToString(Float) ThresholdB))
      (return ThresholdB)
      (else
        (Development|PrintString (Utilities|String|ToString(Float) Input))
        (return Input)))))