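; BP_Dummy2 is a sensor-driven dummy character in the VehicleTwo set whose turning and walk speed respond to a source location.
; MoveForward yaws the actor by an angle computed from the negated source position and moves it along control-rotation forward.
; Walk speed adds averaged inverse-square readings from two socket sensors to a default, subtracts Speciesvelocity and caps the result.
; SpeciesRadius overlaps set or clear Speciesvelocity on nearby BP_InhiDummy actors.
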(event OnComponentBeginOverlap(SpeciesRadius)
  (params (OverlappedComponent :type Primitive%20Component%20Object%20Reference) (OtherActor :type Actor%20Object%20Reference) (OtherComp :type Primitive%20Component%20Object%20Reference) (OtherBodyIndex :type Integer) (bFromSweep :type Boolean) (SweepResult :type Hit%20Result%20Structure%20%28by%20ref%29))
  ;[1 1 1] Overlap Species Code
  (bind _asbp_inhi_dummy (Utilities|Casting|CastToBP_InhiDummy OtherActor))
  (Variables|/Game/BV/VehicleOne/BP_InhiDummy.BP_InhiDummy_C|SetSpeciesvelocity _asbp_inhi_dummy 1e+02))

(event OnComponentEndOverlap(SpeciesRadius)
  (params (OverlappedComponent :type Primitive%20Component%20Object%20Reference) (OtherActor :type Actor%20Object%20Reference) (OtherComp :type Primitive%20Component%20Object%20Reference) (OtherBodyIndex :type Integer))
  ;[1 1 1] Overlap Species Code
  (bind _asbp_inhi_dummy (Utilities|Casting|CastToBP_InhiDummy OtherActor))
  (Variables|/Game/BV/VehicleOne/BP_InhiDummy.BP_InhiDummy_C|SetSpeciesvelocity _asbp_inhi_dummy 0.0))

(event Custom|MoveForward
  (params (SourceLocation :type Vector))
  (bind _maxvelocity (Variables|Default|GetmaxVelocity))
  ;[1 1 1] Forward Movement Setter
  (bind (_yaw _velocity) (CallFunction|GetYawInputPlayerVelocity SourceLocation))
  (if (<= (- (+ (Variables|Default|GetDefaultVelocity) _velocity) (Variables|Default|GetSpeciesvelocity)) _maxvelocity)
    (Variables|Default|SetNewVelocity (- (+ (Variables|Default|GetDefaultVelocity) _velocity) (Variables|Default|GetSpeciesvelocity)))
    (else
      (Variables|Default|SetNewVelocity _maxvelocity)))
  (Class|Actor|AddActorWorldRotation (Math|Rotator|MakeRotator 0.0 0.0 _yaw))
  (Pawn|Input|AddMovementInput (Math|Vector|GetForwardVector (Math|Rotator|MakeRotator 0.0 0.0 (.yaw (Pawn|GetControlRotation :!class /Script/Engine.Pawn)))) 1.0 false)
  (bind _output_get (Variables|/Script/Engine.CharacterMovementComponent|SetMaxWalkSpeed (Variables|Character|GetCharacterMovement) (Variables|Default|GetNewVelocity))))

(fn ConstructionScript)

(fn GetSensorLocations
  (bind _capsulecomponent (Variables|Collision|GetCapsuleComponent))
  (return (Transformation|GetSocketLocation _capsulecomponent "clavicle_out_l") (Transformation|GetSocketLocation _capsulecomponent "clavicle_out_r")))

(fn GetYawInputPlayerVelocity
  (params (sourceLocation :type Vector))
  (bind _returnvalue (Transformation|GetActorLocation))
  (Variables|Default|SetSourceLocation (Math|Vector|NegateVector sourceLocation))
  (bind (_sensor1 _sensor2) (CallFunction|GetSensorLocations))
  (return (* (- (Class|KismetMathLibrary|DegAtan2 (- (.x (Variables|Default|GetSourceLocation)) (.x _returnvalue)) (- (.y (Variables|Default|GetSourceLocation)) (.y _returnvalue))) (.yaw (Transformation|GetActorRotation))) 1.0) (/ (+ (/ 1.0 (Math|Float|Square (/ (Math|Vector|VectorLength (- _sensor1 sourceLocation)) 1.2e+04))) (/ 1.0 (Math|Float|Square (/ (Math|Vector|VectorLength (- _sensor2 sourceLocation)) 1.2e+04)))) (Variables|Default|GetnmrSensor))))