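; BP_LightSourceV1 is a light source actor that drives nearby BP_CarV1 vehicles forward according to their distance from it.
; Each tick it runs a multi-sphere object trace around itself and filters hits by "car" in the display name before casting.
; For each car, it converts the sensor's distance into throttle that rises linearly with proximity across the trace radius, then calls MoveForward on that car.
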(event Custom|ScrubTrace
  ;[1 1 1] Scrub trace
  (bind _output_get (Variables|Default|SetmyLocation (Transformation|GetActorLocation)))
  (bind _outhits (Collision|MultiSphereTraceForObjects _output_get _output_get 3e+03 (Variables|Default|GetObject%20Types) false 0 "None"))
  (for _array_element _outhits
    (if (Utilities|String|Contains (Utilities|GetDisplayName (.HitActor (Collision|BreakHitResult _array_element))) "car")
      (bind _asbp_car_v1 (Utilities|Casting|CastToBP_CarV1 (.HitActor (Collision|BreakHitResult _array_element))))
      (bind _sesonlocation (Default|GetSensorLocation _asbp_car_v1))
      (Variables|Default|SethitLocation _sesonlocation)
      (bind _throttleinput (CallFunction|FindThrottleInput))
      (Default|MoveForward _asbp_car_v1 _throttleinput))))

(event EventTick
  (params (DeltaSeconds :type Float%20%28single-precision%29))
  (CallFunction|ScrubTrace))

(fn ConstructionScript)

(fn FindThrottleInput
  (return (- 1.0 (Math|Float|NormalizetoRange (/ (Math|Vector|VectorLength (- (Variables|Default|GethitLocation) (Variables|Default|GetmyLocation))) 3e+03) 0.0 1.0))))