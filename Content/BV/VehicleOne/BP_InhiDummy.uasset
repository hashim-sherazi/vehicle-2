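; BP_InhiDummy is a character for a VehicleOne agent that moves forward at a speed inhibited by an input value.
; MoveForward adds movement along the control-rotation yaw and sets max walk speed to default velocity plus species velocity, minus the input.
; The SpeciesRadius overlap sets a fixed species velocity boost when a BP_Dummy enters and zeroes it when any one leaves.
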(event OnComponentBeginOverlap(SpeciesRadius)
  (params (OverlappedComponent :type Primitive%20Component%20Object%20Reference) (OtherActor :type Actor%20Object%20Reference) (OtherComp :type Primitive%20Component%20Object%20Reference) (OtherBodyIndex :type Integer) (bFromSweep :type Boolean) (SweepResult :type Hit%20Result%20Structure%20%28by%20ref%29))
  (Utilities|Casting|CastToBP_Dummy OtherActor)
  (Variables|Default|SetSpeciesvelocity 1e+02))

(event OnComponentEndOverlap(SpeciesRadius)
  (params (OverlappedComponent :type Primitive%20Component%20Object%20Reference) (OtherActor :type Actor%20Object%20Reference) (OtherComp :type Primitive%20Component%20Object%20Reference) (OtherBodyIndex :type Integer))
  (Utilities|Casting|CastToBP_Dummy OtherActor)
  (Variables|Default|SetSpeciesvelocity 0.0))

(event Custom|MoveForward
  (params (NewParam :type Float%20%28double-precision%29))
  (Variables|Default|SetNewVelocity (- (+ (Variables|Default|GetSpeciesvelocity) (Variables|Default|GetDefaultVelocity)) NewParam))
  (Pawn|Input|AddMovementInput (Math|Vector|GetForwardVector (Math|Rotator|MakeRotator 0.0 0.0 (.yaw (Pawn|GetControlRotation :!class /Script/Engine.Pawn)))) 1.0 false)
  (Variables|/Script/Engine.CharacterMovementComponent|SetMaxWalkSpeed (Variables|Character|GetCharacterMovement) (Variables|Default|GetNewVelocity)))

(fn ConstructionScript)