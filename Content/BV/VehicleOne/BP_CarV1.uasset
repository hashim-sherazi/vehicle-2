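; Drivable car Blueprint that feeds throttle input to its vehicle movement component and can show an on-screen info readout.
; MoveForward also stores the throttle and, while Info is set, creates UW_CarInfo once and refreshes it with the car's name and stats.
; Clearing Info removes that widget on the next MoveForward event.
; GetSensorLocation exposes the Sensor component's world position.
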(event Custom|MoveForward
  (params (ThrottleInput :type Float%20%28double-precision%29))
  ;[0 0 0] Move Forward
  (Class|ChaosVehicleMovementComponent|SetThrottleInput (Variables|Default|GetVehicleMovementComponent) ThrottleInput)
  ;[1 1 1] WidgetUpdate
  (bind _output_get (Variables|Default|SetThrottle ThrottleInput))
  (if (Variables|Default|Getinfo?)
    (if (Variables|Default|GetinfoUp)
      _
      (else
        (bind _returnvalue (UserInterface|CreateWidget "/Game/BV/UI/UW_CarInfo.UW_CarInfo_C" (Game|GetPlayerController 0)))
        (bind _output_get_2 (Variables|Default|SetcarinfoWidget _returnvalue))
        (UserInterface|Viewport|AddtoViewport _output_get_2 0)
        (Variables|Default|SetinfoUp true)))
    (Variables|/Script/UMG.TextBlock|SetText (Variables|/Game/BV/UI/UW_CarInfo.UW_CarInfo_C|GetThrottle (Variables|Default|GetcarinfoWidget)) (Utilities|Text|ToText(Float) _output_get "HalfToEven"))
    (Variables|/Script/UMG.TextBlock|SetText (Variables|/Game/BV/UI/UW_CarInfo.UW_CarInfo_C|GetAngle (Variables|Default|GetcarinfoWidget)) (Utilities|Text|ToText(Float) (Variables|Default|GetAngle) "HalfToEven"))
    (Variables|/Script/UMG.TextBlock|SetText (Variables|/Game/BV/UI/UW_CarInfo.UW_CarInfo_C|GetNMR (Variables|Default|GetcarinfoWidget)) (Utilities|Text|ToText(Integer) (Variables|Default|GetNMR)))
    (Variables|/Script/UMG.TextBlock|SetText (Variables|/Game/BV/UI/UW_CarInfo.UW_CarInfo_C|GetWeight (Variables|Default|GetcarinfoWidget)) (Utilities|Text|ToText(Float) (Variables|Default|GetWeight) "HalfToEven"))
    (Variables|/Script/UMG.TextBlock|SetText (Variables|/Game/BV/UI/UW_CarInfo.UW_CarInfo_C|GetVehicleName (Variables|Default|GetcarinfoWidget)) (Utilities|Text|ToText(Name) (Variables|Default|GetCarname)))
    (else
      (bind _carinfowidget (Variables|Default|GetcarinfoWidget)
        (:then
          (Widget|RemovefromParent _carinfowidget)
          (Variables|Default|SetinfoUp false))
        (:else)))))

(fn ConstructionScript)

(fn GetSensorLocation
  (return (Transformation|GetWorldLocation (Variables|Default|GetSensor))))