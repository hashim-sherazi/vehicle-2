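; BP_Dummy is a Character-based dummy that moves forward at variable speed and slows nearby BP_InhiDummy actors.
; MoveForward adds its input to a default velocity, subtracts its own Speciesvelocity, caps the result as max walk speed, and moves along control yaw.
; The SpeciesRadius overlap sets the other BP_InhiDummy's Speciesvelocity penalty on entry and clears it on exit.
; A speed debug print is left unconnected.
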(event OnComponentBeginOverlap(SpeciesRadius)
  (params (OverlappedComponent :type Primitive%20Component%20Object%20Reference) (OtherActor :type Actor%20Object%20Reference) (OtherComp :type Primitive%20Component%20Object%20Reference) (OtherBodyIndex :type Integer) (bFromSweep :type Boolean) (SweepResult :type Hit%20Result%20Structure%20%28by%20ref%29))
  ;[1 1 1] Overlap Species Code
  (bind _asbp_inhi_dummy (Utilities|Casting|CastToBP_InhiDummy OtherActor))
  (Variables|/Game/BV/VehicleOne/BP_InhiDummy.BP_InhiDummy_C|SetSpeciesvelocity _asbp_inhi_dummy 1e+02))

(event OnComponentEndOverlap(SpeciesRadius)
  (params (OverlappedComponent :type Primitive%20Component%20Object%20Reference) (OtherActor :type Actor%20Object%20Reference) (OtherComp :type Primitive%20Component%20Object%20Reference) (OtherBodyIndex :type Integer))
  ;[1 1 1] Overlap Species Code
  (bind _asbp_inhi_dummy (Utilities|Casting|CastToBP_InhiDummy OtherActor))
  (Variables|/Game/BV/VehicleOne/BP_InhiDummy.BP_InhiDummy_C|SetSpeciesvelocity _asbp_inhi_dummy 0.0))

(event Custom|MoveForward
  (params (NewParam :type Float%20%28double-precision%29))
  (bind _defaultvelocity (Variables|Default|GetDefaultVelocity))
  (bind _speciesvelocity (Variables|Default|GetSpeciesvelocity))
  (bind _maxvelocity (Variables|Default|GetmaxVelocity))
  (bind _returnvalue (+ _defaultvelocity NewParam))
  (bind _returnvalue_2 (- _returnvalue _speciesvelocity))
  ;[1 1 1] Forward Movement Setter
  (if (<= _returnvalue_2 _maxvelocity)
    (Variables|Default|SetNewVelocity _returnvalue_2)
    (else
      (Variables|Default|SetNewVelocity _maxvelocity)))
  (Pawn|Input|AddMovementInput (Math|Vector|GetForwardVector (Math|Rotator|MakeRotator 0.0 0.0 (.yaw (Pawn|GetControlRotation :!class /Script/Engine.Pawn)))) 1.0 false)
  (bind _output_get (Variables|/Script/Engine.CharacterMovementComponent|SetMaxWalkSpeed (Variables|Character|GetCharacterMovement) (Variables|Default|GetNewVelocity))))

(fn ConstructionScript)