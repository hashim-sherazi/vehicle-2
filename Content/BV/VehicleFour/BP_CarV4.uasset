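; BP_CarV4 is a self-driving, Braitenberg-style car that reacts to nearby actors with "source" in their name, found by a sphere trace every tick.
; Left and right excitatory minus inhibitory sensor groups turn source distance, through ReLU, into one averaged, log-scaled throttle.
; Steering comes separately from the world look-at yaw toward the source.
; An optional widget shows car stats; sigmoid and step activations are unused.
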(event Custom|ScrubTrace
  (bind _returnvalue (Transformation|GetActorLocation))
  (bind _outhits (Collision|MultiSphereTraceForObjects _returnvalue _returnvalue 2.8e+03 (Variables|Default|GetObject%20Types) false 0 "ForDuration" true "(R=0.088195,G=1.000000,B=0.100112,A=1.000000)" "(R=0.263167,G=1.000000,B=0.093465,A=1.000000)" 1.0))
  (for _array_element _outhits
    (if (Utilities|String|Contains (Utilities|GetDisplayName (.HitActor (Collision|BreakHitResult _array_element))) "source")
      (Variables|Default|SethitLocation (Transformation|GetActorLocation (.HitActor (Collision|BreakHitResult _array_element))))
      (bind (_left _right) (CallFunction|GetthrottleInputs))
      (bind _steering (CallFunction|GetSteeringAngle))
      (bind _output_get (Variables|Default|SetAngle _steering))
      (Class|ChaosVehicleMovementComponent|SetSteeringInput (Variables|Default|GetVehicleMovementComponent) _output_get)
      (bind _output_get_2 (Variables|Default|SetThrottle (Math|Float|MapRangeClamped (Math|Float|Log (* (Math|Float|Absolute(Float) (/ (+ _left _right) 2.0)) (Variables|Default|GetThrottleSmoother)) 1e+01) -5.0 5.0 0.0 1.0)))
      (Class|ChaosVehicleMovementComponent|SetThrottleInput (Variables|Default|GetVehicleMovementComponent) _output_get_2)
      ;[1 1 1] WidgetUpdate
      (if (Variables|Default|Getinfo?)
        (if (Variables|Default|GetinfoUp)
          _
          (else
            (bind _returnvalue_2 (UserInterface|CreateWidget "/Game/BV/UI/UW_CarInfo.UW_CarInfo_C" (Game|GetPlayerController 0)))
            (bind _output_get_3 (Variables|Default|SetcarinfoWidget _returnvalue_2))
            (UserInterface|Viewport|AddtoViewport _output_get_3 0)
            (Variables|Default|SetinfoUp true)))
        (Variables|/Script/UMG.TextBlock|SetText (Variables|/Game/BV/UI/UW_CarInfo.UW_CarInfo_C|GetThrottle (Variables|Default|GetcarinfoWidget)) (Utilities|Text|ToText(Float) (Variables|Default|GetThrottle) "HalfToEven"))
        (Variables|/Script/UMG.TextBlock|SetText (Variables|/Game/BV/UI/UW_CarInfo.UW_CarInfo_C|GetAngle (Variables|Default|GetcarinfoWidget)) (Utilities|Text|ToText(Float) (Variables|Default|GetAngle) "HalfToEven"))
        (Variables|/Script/UMG.TextBlock|SetText (Variables|/Game/BV/UI/UW_CarInfo.UW_CarInfo_C|GetNMR (Variables|Default|GetcarinfoWidget)) (Utilities|Text|ToText(Integer) (Variables|Default|GetNMR)))
        (Variables|/Script/UMG.TextBlock|SetText (Variables|/Game/BV/UI/UW_CarInfo.UW_CarInfo_C|GetWeight (Variables|Default|GetcarinfoWidget)) (Utilities|Text|ToText(Float) (Variables|Default|GetWeight) "HalfToEven"))
        (Variables|/Script/UMG.TextBlock|SetText (Variables|/Game/BV/UI/UW_CarInfo.UW_CarInfo_C|GetVehicleName (Variables|Default|GetcarinfoWidget)) (Utilities|Text|ToText(Name) (Variables|Default|GetCarname)))
        (else
          (bind _carinfowidget (Variables|Default|GetcarinfoWidget)
            (:then
              (Widget|RemovefromParent _carinfowidget)
              (Variables|Default|SetinfoUp false))
            (:else)))))))

(event EventTick
  (params (DeltaSeconds :type Float%20%28single-precision%29))
  (Variables|Default|Setcar%20location (Transformation|GetActorLocation))
  (CallFunction|ScrubTrace))

(fn ConstructionScript)

(fn GetSensorinput
  (params (Sensor :type Vector) (ThresholdA :type Float%20%28double-precision%29) (ThresholdB :type Float%20%28double-precision%29))
  ;[1 1 1] Get Sensory input
  (bind _output (CallFunction|ReluFunction (Math|Float|NormalizetoRange (/ (Math|Vector|VectorLength (- (Variables|Default|GethitLocation) Sensor)) 3e+01) 0.0 1.0) (Variables|Default|GetThresholdA)))
  (return _output))

(fn GetthrottleInputs
  ;[1 1 1] Left Throttle Input
  (bind _sensorout (CallFunction|GetSensorinput (Transformation|GetWorldLocation (Variables|Default|GetExciRight1)) 0.1 0.4))
  (bind _sensorout_2 (CallFunction|GetSensorinput (Transformation|GetWorldLocation (Variables|Default|GetExciRight2)) 0.1 0.4))
  (bind _sensorout_3 (CallFunction|GetSensorinput (Transformation|GetWorldLocation (Variables|Default|GetExciRight3)) 0.1 0.4))
  (bind _sensorout_4 (CallFunction|GetSensorinput (Transformation|GetWorldLocation (Variables|Default|GetExciRight4)) 0.1 0.4))
  (bind _sensorout_5 (CallFunction|GetSensorinput (Transformation|GetWorldLocation (Variables|Default|GetExciRight5)) 0.1 0.4))
  (bind _sensorout_6 (CallFunction|GetSensorinput (Transformation|GetWorldLocation (Variables|Default|GetInhiRight1)) 0.1 0.4))
  (bind _sensorout_7 (CallFunction|GetSensorinput (Transformation|GetWorldLocation (Variables|Default|GetInhiRight2)) 0.1 0.4))
  (bind _sensorout_8 (CallFunction|GetSensorinput (Transformation|GetWorldLocation (Variables|Default|GetInhiRight3)) 0.1 0.4))
  ;[1 1 1] Right Throttle Input
  (bind _sensorout_9 (CallFunction|GetSensorinput (Transformation|GetWorldLocation (Variables|Default|GetExciLeft1)) 0.1 0.4))
  (bind _sensorout_10 (CallFunction|GetSensorinput (Transformation|GetWorldLocation (Variables|Default|GetExciLeft2)) 0.1 0.4))
  (bind _sensorout_11 (CallFunction|GetSensorinput (Transformation|GetWorldLocation (Variables|Default|GetExciLeft3)) 0.1 0.4))
  (bind _sensorout_12 (CallFunction|GetSensorinput (Transformation|GetWorldLocation (Variables|Default|GetExciLeft4)) 0.1 0.4))
  (bind _sensorout_13 (CallFunction|GetSensorinput (Transformation|GetWorldLocation (Variables|Default|GetExciLeft5)) 0.1 0.4))
  (bind _sensorout_14 (CallFunction|GetSensorinput (Transformation|GetWorldLocation (Variables|Default|GetInhiLeft1)) 0.1 0.4))
  (bind _sensorout_15 (CallFunction|GetSensorinput (Transformation|GetWorldLocation (Variables|Default|GetInhiLeft2)) 0.1 0.4))
  (bind _sensorout_16 (CallFunction|GetSensorinput (Transformation|GetWorldLocation (Variables|Default|GetInhiLeft3)) 0.1 0.4))
  (return (- (* (/ (+ _sensorout _sensorout_2 _sensorout_3 _sensorout_4 _sensorout_5) 5.0) (Variables|Default|GetExcitatorySmoother)) (* (/ (+ _sensorout_6 _sensorout_7 _sensorout_8) 3.0) (Variables|Default|GetInhiSmoother))) (- (* (/ (+ _sensorout_9 _sensorout_10 _sensorout_11 _sensorout_12 _sensorout_13) 5.0) (Variables|Default|GetExcitatorySmoother)) (* (/ (+ _sensorout_14 _sensorout_15 _sensorout_16) 3.0) (Variables|Default|GetInhiSmoother)))))

(fn GetSteeringAngle
  (return (* (Variables|Default|GetSteeringSmoother) (/ (.yaw (Math|Rotator|FindLookatRotation (Variables|Default|Getcar%20location) (Variables|Default|GethitLocation))) 3.6e+02))))

(fn ReluFunction
  (params (input :type Float%20%28double-precision%29) (Threshold :type Float%20%28double-precision%29))
  (if (< input Threshold)
    (return 0.0)
    (else
      (return input))))

(fn SigmoidFunction
  (params (Input :type Float%20%28double-precision%29))
  (bind _returnvalue (* Input -1.0))
  (bind _returnvalue_2 (Class|KismetMathLibrary|Exp _returnvalue))
  (bind _returnvalue_3 (+ 1.0 _returnvalue_2))
  (bind _returnvalue_4 (/ 1.0 _returnvalue_3))
  (Development|PrintText (Utilities|Text|FormatText "Input {in} output {out}" Input _returnvalue_4))
  (return _returnvalue_4))

(fn StepFunction
  (params (Input :type Float%20%28double-precision%29) (ThresholdA :type Float%20%28double-precision%29) (ThresholdB :type Float%20%28double-precision%29))
  (if (<= Input ThresholdA)
    (Development|PrintString (Utilities|String|ToString(Float) ThresholdA))
    (return ThresholdA)
    (elif (>= Input ThresholdB)
      (Development|PrintString (Utilities|String|ToString(Float) ThresholdB))
      (return ThresholdB)
      (else
        (Development|PrintString (Utilities|String|ToString(Float) Input))
        (return Input)))))